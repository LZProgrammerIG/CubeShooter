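; Hitscan rifle weapon Blueprint that supplies first-person animations for reloading and equipping.
; Its reload and equip events play the animation directly on the player character's first-person mesh, then restore AnimBP mode after a hard-coded delay.
; The fire animation event is empty, with its montage playback logic left disconnected, and no hitscan logic lives in these graphs.
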(event `self.PlayReloadAnimation`
  (bind _playercharacter (`self.PlayerCharacter`))
  (bind _firstpersonmesh (`CubeShooterCharacter.FirstPersonMesh` _playercharacter))
  (`/Engine/EditorBlueprintResources/StandardMacros.IsValid` _firstpersonmesh
    (:`Is Valid`
      (`SkeletalMeshComponent.PlayAnimation` _firstpersonmesh "/Game/Characters/Mannequins/Anims/Rifle/MM_Rifle_Reload.MM_Rifle_Reload" false)
      (`KismetSystemLibrary.Delay` 2.2)
      (`CubeShooterCharacter.SetAnimaModeToAnimBP` _playercharacter))))

(event `self.PlayEquipAnimation`
  (bind _playercharacter (`self.PlayerCharacter`))
  (bind _firstpersonmesh (`CubeShooterCharacter.FirstPersonMesh` _playercharacter))
  (`/Engine/EditorBlueprintResources/StandardMacros.IsValid` _firstpersonmesh
    (:`Is Valid`
      (`SkeletalMeshComponent.PlayAnimation` _firstpersonmesh "/Game/Characters/Mannequins/Anims/Rifle/MM_Rifle_Equip.MM_Rifle_Equip" false)
      (`KismetSystemLibrary.Delay` 1.67)
      (`CubeShooterCharacter.SetAnimaModeToAnimBP` _playercharacter))))

(event `self.PlayFireAnimation`)

(fn `UserConstructionScript`)